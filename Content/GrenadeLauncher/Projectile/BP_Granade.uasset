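; BP_Granade is a grenade launcher projectile that explodes on a fixed fuse after spawning.
; After a short delay from BeginPlay, it spawns a Niagara explosion at the mesh location, fires a RadialForce impulse, plays the blast sound and destroys itself.
; Mesh hits only play a metallic drop sound, started partway into the clip, and do not trigger detonation.
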(event OnComponentHit(StaticMesh)
  (params (HitComponent :type Primitive%20Component%20Object%20Reference) (OtherActor :type Actor%20Object%20Reference) (OtherComp :type Primitive%20Component%20Object%20Reference) (NormalImpulse :type Vector :default "0, 0, 0") (Hit :type Hit%20Result%20Structure%20%28by%20ref%29))
  (Audio|PlaySoundatLocation "/Game/GrenadeLauncher/soundFX/heavy_metal_drop.heavy_metal_drop" (Transformation|GetWorldLocation (Variables|Default|GetStaticMesh)) "0, 0, 0" 1.0 1.0 1.0 0 0 0 0))

(event EventBeginPlay
  (Utilities|FlowControl|Delay 2.0)
  (Niagara|SpawnSystematLocation "/Game/GrenadeLauncher/niagaraFX/N_Explosion.N_Explosion" (Transformation|GetWorldLocation (Variables|Default|GetStaticMesh)))
  (Class|RadialForceComponent|FireImpulse (Variables|Default|GetRadialForce))
  (Audio|PlaySoundatLocation "/Game/GrenadeLauncher/soundFX/SFX_Granade_1.SFX_Granade_1" (Transformation|GetWorldLocation (Variables|Default|GetStaticMesh)) "0, 0, 0" 1.0 1.0 0.0 0 0 0 0)
  (Actor|DestroyActor))

(fn ConstructionScript)